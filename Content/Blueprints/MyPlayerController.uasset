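; MyPlayerController is a player controller that creates the player's HUD and relays respawn requests to the game mode.
; ClientPostLogin waits briefly, then creates a HUDWidget owned by the controller and adds it to the viewport.
; Respawn forwards the Pawn to RespawnServer, which runs on the server and passes the controller and Pawn to MyGameMode's RespawnRunOnServer.
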(event `ClientPostLogin`
  ;[1 1 1] HUD作成
  (`KismetSystemLibrary.Delay` 0.2)
  (bind _returnvalue (`|CreateWidget` "/Game/Blueprints/HUDWidget.HUDWidget_C" self))
  (`UserWidget.AddToViewport` _returnvalue 0))

(event `Respawn`
  (params (Pawn :type "/Game/Blueprints/MyPlayerCharacter Object Reference"))
  ;[1 1 1] リスポーンをサーバーで呼ぶ
  (`self.RespawnServer` Pawn))

(event `RespawnServer`
  (params (Pawn :type "/Game/Blueprints/MyPlayerCharacter Object Reference"))
  ;[1 1 1] サーバー上でリスポーンを実行
  (bind _asmy_game_mode (cast `/Game/Blueprints/MyGameMode` (`GameplayStatics.GetGameMode`)))
  (`/Game/Blueprints/MyGameMode.Respawn RunOnServer` _asmy_game_mode self Pawn))

(fn `UserConstructionScript`)